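; Player character for a 2D flipbook game with wolf enemies, handling movement, jumping, sword attacks, damage and death.
; Enhanced Input drives actions gated by state flags, with delays timing animations and cooldowns and a velocity polling loop detecting landing.
; Tick fires HitCheck once on attack frame 3, damaging wolves overlapping the Sword with effect and sound.
; Damage is ignored while attacking, jumping or recently hit; zero health plays death, then destroys the actor.
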(event `self.ReceiveBeginPlay`
  (`|ExecutionSequence`
    (:`then_0`
      (bind _asbp_player_controller (cast `/Game/BLueprints/BP_PlayerController` (`self.GetController`)))
      (`EnhancedInputSubsystemInterface.AddMappingContext` (pcsubsystem `EnhancedInputLocalPlayerSubsystem` _asbp_player_controller) "/Game/BLueprints/IMC_Default.IMC_Default" 0 (struct)))
    (:`then_1`
      (bind _returnvalue (`|CreateWidget` "/Game/BLueprints/HUD.HUD_C"))
      (`UserWidget.AddToViewport` _returnvalue 0))))

(event `EnhancedInput|/Game/BLueprints/IA_Movement`
  (params (ActionValue :type "Float (double-precision)") (ElapsedSeconds :type "Float (double-precision)") (TriggeredSeconds :type "Float (double-precision)") (InputAction :type "InputAction Object Reference" :default "/Game/BLueprints/IA_Movement.IA_Movement"))
  (:`Triggered`
    (if (`self.IsTakingDamage`)
      _
      (elif (`self.Is_Attacking`)
        _
        (elif (not (`self.Is_Jumping`))
          (`self.AddMovementInput` (`self.GetActorForwardVector`) ActionValue)
          (`PaperFlipbookComponent.SetFlipbook` (`self.Sprite`) "/Game/Assets/Player_Run_Anni.Player_Run_Anni")
          (if (> ActionValue 0.0)
            (`SceneComponent.K2_SetWorldRotation` :`self` (`self.Sprite`))
            (else
              (`SceneComponent.K2_SetWorldRotation` (`self.Sprite`) (struct :`Yaw` 180.0) false false)))))))
  (:`Completed`
    (if (`self.IsTakingDamage`)
      _
      (elif (`self.Is_Attacking`)
        _
        (elif (not (`self.Is_Jumping`))
          (`PaperFlipbookComponent.SetFlipbook` (`self.Sprite`) "/Game/Assets/Player_Idle_Anni.Player_Idle_Anni"))))))

(event `EnhancedInput|/Game/BLueprints/IA_Jump`
  (params (ActionValue :type "Float (double-precision)") (ElapsedSeconds :type "Float (double-precision)") (TriggeredSeconds :type "Float (double-precision)") (InputAction :type "InputAction Object Reference" :default "/Game/BLueprints/IA_Jump.IA_Jump"))
  (bind _sprite (`self.Sprite`))
  (:`Triggered`
    (if (`self.IsTakingDamage`)
      _
      (elif (`self.Is_Attacking`)
        _
        (elif (not (`self.Is_Jumping`))
          (set `self.Is_Jumping` true)
          (`self.Jump`)
          (`PaperFlipbookComponent.SetLooping` _sprite false)
          (`PaperFlipbookComponent.SetFlipbook` _sprite "/Game/Assets/Player_Jump_Anni.Player_Jump_Anni")
          (`KismetSystemLibrary.Delay` 0.04)
          (if (== (`.Z` (`KismetMathLibrary.BreakVector3f` (`self.GetVelocity`))) 0.0) :!label _label
            (`PaperFlipbookComponent.SetLooping` _sprite true)
            (`PaperFlipbookComponent.Play` _sprite)
            (`PaperFlipbookComponent.SetFlipbook` _sprite "/Game/Assets/Player_Idle_Anni.Player_Idle_Anni")
            (set `self.Is_Jumping` false)
            (else
              (`KismetSystemLibrary.Delay` 0.01)
              (goto _label))))))))

(event `EnhancedInput|/Game/BLueprints/IA_Attack`
  (params (ActionValue :type Boolean) (ElapsedSeconds :type "Float (double-precision)") (TriggeredSeconds :type "Float (double-precision)") (InputAction :type "InputAction Object Reference" :default "/Game/BLueprints/IA_Attack.IA_Attack"))
  (bind _sprite (`self.Sprite`))
  (:`Triggered`
    (if (`self.IsDead`)
      _
      (elif (`self.IsTakingDamage`)
        _
        (elif (`self.Is_Jumping`)
          _
          (elif (not (`self.IsAttackCD`))
            (set `self.IsAttackCD` true)
            (set `self.Is_Attacking` true)
            (`PaperFlipbookComponent.SetLooping` _sprite false)
            (`PaperFlipbookComponent.SetFlipbook` _sprite "/Game/Assets/Player_Attack_Anni.Player_Attack_Anni")
            (`KismetSystemLibrary.Delay` 0.6)
            (`PaperFlipbookComponent.SetLooping` _sprite true)
            (`PaperFlipbookComponent.Play` _sprite)
            (`PaperFlipbookComponent.SetFlipbook` _sprite "/Game/Assets/Player_Idle_Anni.Player_Idle_Anni")
            (set `self.Is_Attacking` false)
            (`KismetSystemLibrary.Delay` 0.8)
            (set `self.IsAttackCD` false)
            (`self.ResetAttack`)))))))

(event `ResetAttack`
  (goto _label_2 :!via `Reset`))

(event `self.ReceiveTick`
  (params (DeltaSeconds :type "Float (single-precision)"))
  (if (`self.IsDead`)
    _
    (elif (`self.Is_Attacking`)
      (if (== (`PaperFlipbookComponent.GetPlaybackPositionInFrames` (`self.Sprite`)) 3)
        (`/Engine/EditorBlueprintResources/StandardMacros.DoOnce` false :!label _label_2
          (:`Completed`
            (`self.HitCheck`)))))))

(event `self.ReceiveAnyDamage`
  (params (Damage :type "Float (single-precision)") (DamageType :type "DamageType Object Reference") (InstigatedBy :type "Controller Object Reference") (DamageCauser :type "Actor Object Reference"))
  (bind _sprite (`self.Sprite`))
  (bind _sprite_2 (`self.Sprite`))
  (`KismetSystemLibrary.PrintString` (`KismetStringLibrary.Conv_DoubleToString` Damage))
  (if (`self.Is_Attacking`)
    _
    (elif (`self.TookDamageRecantly`)
      _
      (elif (not (`self.Is_Jumping`))
        (set `self.IsTakingDamage` true)
        (set `self.TookDamageRecantly` true)
        (bind _output_get (set `self.Health` (- (`self.Health`) Damage)))
        (`KismetSystemLibrary.Delay` 0.1)
        (if (<= _output_get 0.0)
          (`KismetSystemLibrary.PrintString` "ojoj ale mi sie umarło teraz już bez hp jestem")
          (set `self.IsDead` true)
          (`/Engine/EditorBlueprintResources/StandardMacros.DoOnce` false
            (:`Completed`
              (`PrimitiveComponent.SetCollisionEnabled` (`self.CapsuleComponent`) "NoCollision")
              (`PaperFlipbookComponent.SetLooping` _sprite_2 false)
              (`PaperFlipbookComponent.Play` (`self.Sprite`))
              (`PaperFlipbookComponent.SetFlipbook` _sprite_2 "/Game/Assets/Player_Dead_Anni.Player_Dead_Anni")
              (`KismetSystemLibrary.Delay` 5.0)
              (`self.K2_DestroyActor`)))
          (else
            (`KismetSystemLibrary.PrintString` "ale dostałem")
            (`PaperFlipbookComponent.SetLooping` (`self.Sprite`) false)
            (`PaperFlipbookComponent.SetFlipbook` (`self.Sprite`) "/Game/Assets/Player_Damage_Taken_Anni.Player_Damage_Taken_Anni")
            (`KismetSystemLibrary.Delay` 0.6)
            (`PaperFlipbookComponent.SetLooping` _sprite true)
            (`PaperFlipbookComponent.Play` _sprite)
            (`PaperFlipbookComponent.SetFlipbook` (`self.Sprite`) "/Game/Assets/Player_Idle_Anni.Player_Idle_Anni")
            (set `self.IsTakingDamage` false)
            (`KismetSystemLibrary.Delay` 0.3)
            (set `self.TookDamageRecantly` false)))))))

(fn `HitCheck`
  (for _array_element (`PrimitiveComponent.GetOverlappingActors` (`self.Sword`) "/Game/BLueprints/BP_Wolf.BP_Wolf_C")
    (if (!= _array_element self)
      (`GameplayStatics.ApplyDamage` _array_element (`self.Base Damage`))
      (set `self.HitSomething` true)))
  (if (`self.HitSomething`)
    (`GameplayStatics.SpawnEmitterAtLocation` "/Game/Realistic_Starter_VFX_Pack_Vol2/Particles/Hit/P_Default.P_Default" (`SceneComponent.GetSocketLocation` (`self.Sprite`) "HitPos") (struct) (0.4 1.0 0.4))
    (set `self.HitSomething` false)
    (`GameplayStatics.PlaySound2D` "/Game/SoundEffect/mixkit-sword-cutting-flesh-2788.mixkit-sword-cutting-flesh-2788" 1.0 1.0 0.0 null null)
    (else
      (`GameplayStatics.PlaySound2D` "/Game/SoundEffect/mixkit-fast-sword-whoosh-2792.mixkit-fast-sword-whoosh-2792" 1.0 1.0 0.0 null null))))

(fn `UserConstructionScript`)