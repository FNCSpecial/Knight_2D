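; BP_Shop is an interactable shop that opens only when no BP_Wolf actors remain in the level.
; Interact blends the view to the shop, adds the Shop_UI widget with UI-only input and mouse cursor, and hides the player character; otherwise it prints that enemies are alive.
; Box overlap events toggle a TextRender prompt for BP_Player.
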(event `/Game/BLueprints/Interact_Interface.Interact`
  (bind _returnvalue (`GameplayStatics.GetPlayerController` 0))
  (bind _outactors (`GameplayStatics.GetAllActorsOfClass` "/Game/BLueprints/Mobs-Objects/BP_Wolf.BP_Wolf_C"))
  (bind _output_get (set `self.Out Actors_0` _outactors))
  (if (== (`KismetArrayLibrary.Array_Length` _output_get) 0)
    (`KismetSystemLibrary.PrintString` "Interakcja z sklepem")
    (`PlayerController.SetViewTargetWithBlend` (`GameplayStatics.GetPlayerController` 0) self 0.0 "VTBlend_Linear" 0.0 false)
    (bind _returnvalue_2 (`|CreateWidget` "/Game/UI/Shop_UI.Shop_UI_C"))
    (`UserWidget.AddToViewport` _returnvalue_2 0)
    (`WidgetBlueprintLibrary.SetInputMode_UIOnlyEx` _returnvalue _returnvalue_2)
    (set `PlayerController.bShowMouseCursor` true _returnvalue)
    (`self.SetActorHiddenInGame` (`GameplayStatics.GetPlayerCharacter` 0) true)
    (else
      (`KismetSystemLibrary.PrintString` "wrogowie zyja"))))

(event `self.Box.OnComponentBeginOverlap`
  (params (OverlappedComponent :type "PrimitiveComponent Object Reference") (OtherActor :type "Actor Object Reference") (OtherComp :type "PrimitiveComponent Object Reference") (OtherBodyIndex :type Integer) (bFromSweep :type Boolean) (SweepResult :type "HitResult Structure (by ref)"))
  (cast `/Game/BLueprints/Player/BP_Player` OtherActor)
  (`SceneComponent.SetHiddenInGame` (`self.TextRender`) false false))

(event `self.Box.OnComponentEndOverlap`
  (params (OverlappedComponent :type "PrimitiveComponent Object Reference") (OtherActor :type "Actor Object Reference") (OtherComp :type "PrimitiveComponent Object Reference") (OtherBodyIndex :type Integer))
  (cast `/Game/BLueprints/Player/BP_Player` OtherActor)
  (`SceneComponent.SetHiddenInGame` (`self.TextRender`) true false))

(fn `UserConstructionScript`)