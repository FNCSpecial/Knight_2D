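; BP_Wolf is a flipbook-animated enemy mob that roams, hunts the player on sight or when damaged, and bites.
; Boolean states and recursive AIMoveTo events drive the roam, chase and attack loop.
; Tick updates the camera-facing health bar and triggers a DoOnce-gated bite overlap check during attacks.
; Death awards XP and coins before delayed destruction, and a top trigger pushes away players falling onto it.
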(event `self.ReceiveAnyDamage`
  (params (Damage :type "Float (single-precision)") (DamageType :type "DamageType Object Reference") (InstigatedBy :type "Controller Object Reference") (DamageCauser :type "Actor Object Reference"))
  (bind _sprite (`self.Sprite`))
  ;[1 1 1] Death / damage apply
  (bind _output_get (set `self.Health` (- (`self.Health`) Damage)))
  (if (<= _output_get 0.0)
    (set `self.IsDead` true)
    (set `self.IsAttacking` false)
    (set `self.IsHunting` false)
    (set `self.IsRoaming` false)
    (`|ExecutionSequence`
      (:`then_0`
        (`/Engine/EditorBlueprintResources/StandardMacros.DoOnce` false
          (:`Completed`
            (`ActorComponent.K2_DestroyComponent` (`self.PawnSensing`))
            (`PrimitiveComponent.SetCollisionEnabled` (`self.CapsuleComponent`) "NoCollision")
            (`PrimitiveComponent.SetCollisionEnabled` (`self.Bite`) "NoCollision")
            (`PrimitiveComponent.SetCollisionEnabled` (`self.Top_wolf`) "NoCollision")
            (`PaperFlipbookComponent.SetLooping` (`self.Sprite`) false)
            (`PaperFlipbookComponent.SetFlipbook` _sprite "/Game/Assets/Wolf_Death_Anni.Wolf_Death_Anni")
            (`PaperFlipbookComponent.Play` _sprite)
            (`KismetSystemLibrary.Delay` 3.0)
            (`self.K2_DestroyActor`))))
      (:`then_1`
        (bind _asbp_player (cast `/Game/BLueprints/Player/BP_Player` (`GameplayStatics.GetPlayerCharacter` 0)))
        (set `/Game/BLueprints/Player/BP_Player.XP` (+ (`/Game/BLueprints/Player/BP_Player.XP` _asbp_player) 100) _asbp_player)
        (set `/Game/BLueprints/Player/BP_Player.Coin` (+ (`/Game/BLueprints/Player/BP_Player.Coin` _asbp_player) 10) _asbp_player)))
    (else
      (set `self.IsAttacking` false)
      (set `self.IsRoaming` false)
      (set `self.IsHunting` true)
      (`self.FollowPlayer`))))

(event `self.ReceiveBeginPlay`
  (if (not (`self.IsDead`))
    (`self.Roam`)))

(event `ResetAttack`
  (goto _label_2 :!via `Reset`))

(event `Roam`
  (bind _returnvalue (or (`self.IsDead`) (`self.IsHunting`)))
  (if (not (or (`self.IsDead`) (`self.IsRoaming`) (`self.IsHunting`)))
    (set `CharacterMovementComponent.MaxWalkSpeed` (`self.Speed_roam`) (`self.CharacterMovement`))
    (`PaperFlipbookComponent.SetFlipbook` (`self.Sprite`) "/Game/Assets/Wolf_Walk_Anni.Wolf_Walk_Anni")
    (set `self.IsRoaming` true)
    (`|AIMoveTo` self (`NavigationSystemV1.K2_GetRandomReachablePointInRadius` (`self.K2_GetActorLocation`) 200.0 null null) null
      (:`OnSuccess`
        (if (not _returnvalue)
          (`PaperFlipbookComponent.SetFlipbook` (`self.Sprite`) "/Game/Assets/Wolf_Idle_Anni.Wolf_Idle_Anni")
          (set `self.IsRoaming` false :!label _label)
          (`KismetSystemLibrary.Delay` 3.0)
          (`self.Roam`)))
      (:`OnFail`
        (if (not _returnvalue)
          (`PaperFlipbookComponent.SetFlipbook` (`self.Sprite`) "/Game/Assets/Wolf_Idle_Anni.Wolf_Idle_Anni")
          (goto _label))))))

(event `self.ReceiveTick`
  (params (DeltaSeconds :type "Float (single-precision)"))
  (bind _hp_bar_widget (`self.HP_bar_widget`))
  (`|ExecutionSequence`
    (:`then_0`
      (if (`self.IsDead`)
        (set `self.IsHunting` false)
        (elif (and (`self.IsHunting`) (`self.IsAttacking`) (== (`PaperFlipbookComponent.GetPlaybackPositionInFrames` (`self.Sprite`)) 0))
          (if true
            (`/Engine/EditorBlueprintResources/StandardMacros.DoOnce` false :!label _label_2
              (:`Completed`
                (`self.HitCheck`)))))))
    (:`then_1`
      (bind _aswb_health_bar (cast `/Game/UI/WB_HealthBar` (`WidgetComponent.GetWidget` (`self.HP_bar_widget`))))
      (`ProgressBar.SetPercent` (`/Game/UI/WB_HealthBar.HealthBar_Mobs` _aswb_health_bar) (/ (`self.Health`) 100.0))
      (`SceneComponent.K2_SetWorldRotation` _hp_bar_widget (`KismetMathLibrary.FindLookAtRotation` (`SceneComponent.K2_GetComponentLocation` _hp_bar_widget) (`SceneComponent.K2_GetComponentLocation` (`PlayerCameraManager.TransformComponent` (`GameplayStatics.GetPlayerCameraManager` 0)))) false false))))

(event `self.PawnSensing.OnSeePawn`
  (params (Pawn :type "Pawn Object Reference"))
  (if (`self.IsDead`)
    _
    (elif (not (`self.IsHunting`))
      (`KismetSystemLibrary.PrintString` "widze")
      (bind _asbp_player (cast `/Game/BLueprints/Player/BP_Player` (`GameplayStatics.GetPlayerCharacter` 0)))
      (if (`/Game/BLueprints/Player/BP_Player.IsDead` _asbp_player)
        (if (not (`self.IsDead`))
          (set `self.IsHunting` false)
          (`self.Roam`))
        (elif (not (`self.IsDead`))
          (set `self.IsHunting` true)
          (`self.FollowPlayer`))))))

(event `FollowPlayer`
  (bind _sprite (`self.Sprite`))
  (if (`self.IsAttacking`)
    _
    (elif (`self.IsDead`)
      _
      (elif (`self.IsHunting`)
        (`PaperFlipbookComponent.SetFlipbook` (`self.Sprite`) "/Game/Assets/Wolf_Walk_Anni.Wolf_Walk_Anni")
        (set `CharacterMovementComponent.MaxWalkSpeed` (`self.speed_hunt`) (`self.CharacterMovement`))
        (`|AIMoveTo` self (0.0 0.0 0.0) (`GameplayStatics.GetPlayerCharacter` 0)
          (:`OnSuccess`
            (set `self.IsAttacking` true)
            (if (not (`self.IsDead`))
              (`PaperFlipbookComponent.SetLooping` (`self.Sprite`) false)
              (`PaperFlipbookComponent.SetFlipbook` (`self.Sprite`) "/Game/Assets/Wolf_Attack_Anni.Wolf_Attack_Anni")
              (`KismetSystemLibrary.Delay` 1.0)
              (if (not (`self.IsDead`))
                (`PaperFlipbookComponent.SetLooping` _sprite true)
                (`PaperFlipbookComponent.SetFlipbook` (`self.Sprite`) "/Game/Assets/Wolf_Walk_Anni.Wolf_Walk_Anni")
                (`PaperFlipbookComponent.Play` _sprite)
                (set `self.IsAttacking` false)
                (`self.ResetAttack`)
                (bind _asbp_player (cast `/Game/BLueprints/Player/BP_Player` (`GameplayStatics.GetPlayerCharacter` 0)))
                (if (`/Game/BLueprints/Player/BP_Player.IsDead` _asbp_player)
                  (set `self.IsHunting` false)
                  (`self.Roam`)
                  (else
                    (`self.FollowPlayer`))))))
          (:`OnFail`
            (bind _asbp_player_2 (cast `/Game/BLueprints/Player/BP_Player` (`GameplayStatics.GetPlayerCharacter` 0)))
            (if (`/Game/BLueprints/Player/BP_Player.IsDead` _asbp_player_2)
              (set `self.IsHunting` false)
              (if (not (`self.IsDead`))
                (`self.Roam`))
              (elif (not (`self.IsDead`))
                (`self.FollowPlayer`)))))))))

(event `self.Top_wolf.OnComponentBeginOverlap`
  (params (OverlappedComponent :type "PrimitiveComponent Object Reference") (OtherActor :type "Actor Object Reference") (OtherComp :type "PrimitiveComponent Object Reference") (OtherBodyIndex :type Integer) (bFromSweep :type Boolean) (SweepResult :type "HitResult Structure (by ref)"))
  (bind _asbp_player (cast `/Game/BLueprints/Player/BP_Player` (`GameplayStatics.GetPlayerCharacter` 0)))
  (bind (_returnvalue_x _returnvalue_y _returnvalue_z) (`KismetMathLibrary.BreakVector` (`self.GetVelocity` _asbp_player)))
  (if (and (== (`GameplayStatics.GetObjectClass` OtherActor) "/Game/BLueprints/Player/BP_Player.BP_Player_C") (< _returnvalue_z 0.0))
    (`/Game/BLueprints/Player/BP_Player.Push Away` _asbp_player)))

(fn `HitCheck`
  (for _array_element (`PrimitiveComponent.GetOverlappingActors` (`self.Bite`) "/Game/BLueprints/Player/BP_Player.BP_Player_C")
    (if (!= _array_element self)
      (`GameplayStatics.ApplyDamage` _array_element (`self.damage_wolf`))
      (`KismetSystemLibrary.PrintString` "Wilk zadal obrazenia"))))

(fn `UserConstructionScript`)