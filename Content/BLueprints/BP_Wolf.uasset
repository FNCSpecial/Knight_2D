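; BP_Wolf is a flipbook-animated enemy that roams, chases the player and bites.
; It wanders to random nearby reachable points until PawnSensing sees a pawn, then follows the player character with AIMoveTo and attacks on arrival.
; Tick watches for attack frame 2 to run a once-per-attack HitCheck, damaging players overlapping Bite.
; At zero health it disables sensing and collision, plays a death animation, then destroys itself.
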(event `self.ReceiveAnyDamage`
  (params (Damage :type "Float (single-precision)") (DamageType :type "DamageType Object Reference") (InstigatedBy :type "Controller Object Reference") (DamageCauser :type "Actor Object Reference"))
  (bind _sprite (`self.Sprite`))
  ;[1 1 1] Death / damage apply
  (`KismetSystemLibrary.PrintString` (`KismetStringLibrary.Conv_DoubleToString` Damage))
  (bind _output_get (set `self.Health` (- (`self.Health`) Damage)))
  (if (<= _output_get 0.0)
    (set `self.IsDead` true)
    (set `self.IsHunting` false)
    (set `self.IsRoaming` false)
    (`/Engine/EditorBlueprintResources/StandardMacros.DoOnce` false
      (:`Completed`
        (`ActorComponent.K2_DestroyComponent` (`self.PawnSensing`))
        (`PrimitiveComponent.SetCollisionEnabled` (`self.CapsuleComponent`) "NoCollision")
        (`PaperFlipbookComponent.SetLooping` _sprite false)
        (`PaperFlipbookComponent.Play` (`self.Sprite`))
        (`PaperFlipbookComponent.SetFlipbook` _sprite "/Game/Assets/Wolf_Death_Anni.Wolf_Death_Anni")
        (`KismetSystemLibrary.Delay` 5.0)
        (`self.K2_DestroyActor`)))))

(event `self.ReceiveBeginPlay`
  (if (not (`self.IsDead`))
    (`self.Roam`)))

(event `Roam`
  (if (`self.IsRoaming`)
    _
    (elif (`self.IsHunting`)
      _
      (elif (not (`self.IsDead`))
        (`PaperFlipbookComponent.SetFlipbook` (`self.Sprite`) "/Game/Assets/Wolf_Walk_Anni.Wolf_Walk_Anni")
        (set `self.IsRoaming` true)
        (`|AIMoveTo` self (`NavigationSystemV1.K2_GetRandomReachablePointInRadius` (`self.K2_GetActorLocation`) 200.0 null null) null
          (:`OnSuccess`
            (`PaperFlipbookComponent.SetFlipbook` (`self.Sprite`) "/Game/Assets/Wolf_Idle_Anni.Wolf_Idle_Anni")
            (`KismetSystemLibrary.Delay` 3.0)
            (set `self.IsRoaming` false)
            (if (not (`self.IsDead`))
              (`self.Roam`)))
          (:`OnFail`
            (`PaperFlipbookComponent.SetFlipbook` (`self.Sprite`) "/Game/Assets/Wolf_Idle_Anni.Wolf_Idle_Anni")
            (`KismetSystemLibrary.Delay` 3.0)
            (set `self.IsRoaming` false)
            (if (not (`self.IsDead`))
              (`self.Roam`))))))))

(event `ResetAttack`
  (goto _label :!via `Reset`))

(event `self.ReceiveTick`
  (params (DeltaSeconds :type "Float (single-precision)"))
  (if (`self.IsDead`)
    (set `self.IsHunting` false)
    (elif (`self.IsHunting`)
      (if (`self.IsAttacking`)
        (if (== (`PaperFlipbookComponent.GetPlaybackPositionInFrames` (`self.Sprite`)) 2)
          (`/Engine/EditorBlueprintResources/StandardMacros.DoOnce` false :!label _label
            (:`Completed`
              (`self.HitCheck`))))))))

(event `self.PawnSensing.OnSeePawn`
  (params (Pawn :type "Pawn Object Reference"))
  (if (not (`self.IsDead`))
    (`KismetSystemLibrary.PrintString` "widze")
    (set `self.IsHunting` true)
    (`self.FollowPlayer`)))

(event `FollowPlayer`
  (bind _sprite (`self.Sprite`))
  (if (`self.IsAttacking`)
    _
    (elif (`self.IsDead`)
      _
      (elif (`self.IsHunting`)
        (`PaperFlipbookComponent.SetFlipbook` (`self.Sprite`) "/Game/Assets/Wolf_Walk_Anni.Wolf_Walk_Anni")
        (`|AIMoveTo` self (0.0 0.0 0.0) (`GameplayStatics.GetPlayerCharacter` 0)
          (:`OnSuccess`
            (set `self.IsAttacking` true)
            (`PaperFlipbookComponent.SetLooping` (`self.Sprite`) false)
            (`PaperFlipbookComponent.SetFlipbook` (`self.Sprite`) "/Game/Assets/Wolf_Attack_Anni.Wolf_Attack_Anni")
            (`KismetSystemLibrary.Delay` 1.0)
            (if (not (`self.IsDead`))
              (`PaperFlipbookComponent.SetLooping` _sprite true)
              (`PaperFlipbookComponent.Play` _sprite)
              (`PaperFlipbookComponent.SetFlipbook` (`self.Sprite`) "/Game/Assets/Wolf_Walk_Anni.Wolf_Walk_Anni")
              (set `self.IsAttacking` false)
              (`self.ResetAttack`)
              (`self.FollowPlayer`)))
          (:`OnFail`
            (`self.FollowPlayer`)))))))

(fn `HitCheck`
  (for _array_element (`PrimitiveComponent.GetOverlappingActors` (`self.Bite`) "/Game/BLueprints/BP_Player.BP_Player_C")
    (if (!= _array_element self)
      (`GameplayStatics.ApplyDamage` _array_element (`self.damage_wolf`))
      (`KismetSystemLibrary.PrintString` "ale mu zajebałem"))))

(fn `UserConstructionScript`)